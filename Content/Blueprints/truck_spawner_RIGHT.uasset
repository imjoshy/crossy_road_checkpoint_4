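; Right-side truck spawner actor that feeds Truck_1 vehicles into the level at irregular intervals.
; BeginPlay picks one random negative speed Multiplier, which is passed to every truck it spawns.
; Tick doubles as the spawn timer, re-randomizing its own interval to a few seconds on each run.
; Each tick also destroys the spawner once the player is over 500 units past it along X.
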(event `self.ReceiveBeginPlay`
  (`self.SetActorTickInterval` (select `int` (`KismetMathLibrary.RandomIntegerInRange` 0 2) :`0` 2.0 :`1` 3.0 :`2` 4.0 :!type "Float (single-precision)"))
  (set `self.mult` (select `int` (`KismetMathLibrary.RandomIntegerInRange` 0 2) :`0` -2 :`1` -3 :`2` -4)))

(event `self.ReceiveTick`
  (params (DeltaSeconds :type "Float (single-precision)"))
  (bind _returnvalue_x (`KismetMathLibrary.BreakVector` (`self.K2_GetActorLocation`)))
  (bind (_returnvalue_x_2 _returnvalue_y) (`KismetMathLibrary.BreakVector` (`self.K2_GetActorLocation`)))
  (bind _returnvalue_x_3 (`KismetMathLibrary.BreakVector` (`self.K2_GetActorLocation`)))
  (bind _returnvalue_x_4 (`KismetMathLibrary.BreakVector` (`self.K2_GetActorLocation` (`GameplayStatics.GetPlayerCharacter` 0))))
  (bind _returnvalue_x_5 (`KismetMathLibrary.BreakVector` (`self.K2_GetActorLocation` (`GameplayStatics.GetPlayerCharacter` 0))))
  (`self.SetActorTickInterval` (select `int` (`KismetMathLibrary.RandomIntegerInRange` 0 3) :`0` 1.0 :`1` 2.0 :`2` 3.0 :`3` 4.0 :!type "Float (single-precision)"))
  (`|ExecutionSequence`
    (:`then_0`
      (bind _returnvalue (`|SpawnActorFromClass` "/Game/Blueprints/truck_1.truck_1_C" (`KismetMathLibrary.MakeTransform` (`KismetMathLibrary.MakeVector` _returnvalue_x_2 _returnvalue_y -20.0) (struct :`Yaw` 90.0 :`Roll` 90.0) (25.0 25.0 25.0)) "Undefined" "OverrideRootScale" null null))
      (set `self.truck_ref` _returnvalue)
      (set `/Game/Blueprints/truck_1.multiplier` (`KismetMathLibrary.Conv_IntToDouble` (`self.mult`)) (`self.truck_ref`)))
    (:`then_1`
      (if (and (< _returnvalue_x _returnvalue_x_5) (> (- (`KismetMathLibrary.Abs` _returnvalue_x_4) (`KismetMathLibrary.Abs` _returnvalue_x_3)) 500.0))
        (`self.K2_DestroyActor`)))))

(fn `UserConstructionScript`)