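; Rock obstacle actor that removes itself once the player has moved past it.
; Each Tick it compares its X location with player character 0 and destroys itself when it is behind and the absolute X values differ by more than 1000 units.
; BeginPlay, overlap and construction script are empty.
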(event `self.ReceiveTick`
  (params (DeltaSeconds :type "Float (single-precision)"))
  (bind _returnvalue_x (`KismetMathLibrary.BreakVector` (`self.K2_GetActorLocation`)))
  (bind _returnvalue_x_2 (`KismetMathLibrary.BreakVector` (`self.K2_GetActorLocation`)))
  (bind _returnvalue_x_3 (`KismetMathLibrary.BreakVector` (`self.K2_GetActorLocation` (`GameplayStatics.GetPlayerCharacter` 0))))
  (bind _returnvalue_x_4 (`KismetMathLibrary.BreakVector` (`self.K2_GetActorLocation` (`GameplayStatics.GetPlayerCharacter` 0))))
  (if (and (< _returnvalue_x _returnvalue_x_4) (> (- (`KismetMathLibrary.Abs` _returnvalue_x_3) (`KismetMathLibrary.Abs` _returnvalue_x_2)) 1000.0))
    (`self.K2_DestroyActor`)))

(fn `UserConstructionScript`)