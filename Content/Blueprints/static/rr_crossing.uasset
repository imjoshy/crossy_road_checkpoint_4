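; Railroad crossing signal that flashes two lights and plays audio while a train is in its trigger zone.
; Trigger overlaps with train actors are counted, so the warning stops only when the count returns to zero.
; Tick replays a timeline that alternates emissive strength on two dynamic materials, dimming both when idle.
; Tick also destroys the actor once the player is sufficiently past it along X.
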(event `self.ReceiveBeginPlay`
  (`|ExecutionSequence`
    (:`then_0`
      ;[1 1 1] no sound to start
      (`AudioComponent.Stop` (`self.Audio`)))
    (:`then_1`
      ;[1 1 1] start both L and R emissions at 0.1 (glowing but barely visible)  https://forums.unrealengine.com/development-discussion/blueprint-visual-scripting/6650-scalar-paramaters-in-blueprints
      (bind _returnvalue (`PrimitiveComponent.CreateDynamicMaterialInstance` (`self.Cube`) 0 "/Game/Assets/rr_emissive_mat_Inst.rr_emissive_mat_Inst" "None"))
      (bind _output_get (set `self.emissive_mat` _returnvalue))
      (`MaterialInstanceDynamic.SetScalarParameterValue` _output_get "emissive_strength" (`self.dim`)))
    (:`then_2`
      (bind _returnvalue_2 (`PrimitiveComponent.CreateDynamicMaterialInstance` (`self.Cube1`) 0 "/Game/Assets/rr_emissive_mat_Inst.rr_emissive_mat_Inst" "None"))
      (bind _output_get_2 (set `self.emissive_mat_2` _returnvalue_2))
      (`MaterialInstanceDynamic.SetScalarParameterValue` _output_get_2 "emissive_strength" (`self.dim`)))))

(event `self.trigger_zone.OnComponentBeginOverlap`
  (params (OverlappedComponent :type "PrimitiveComponent Object Reference") (OtherActor :type "Actor Object Reference") (OtherComp :type "PrimitiveComponent Object Reference") (OtherBodyIndex :type Integer) (bFromSweep :type Boolean) (SweepResult :type "HitResult Structure (by ref)"))
  ;[1 1 1] trigger_zone checks if train's Box collision component overlaps
  (cast `/Game/Blueprints/train` OtherActor)
  (set `self.approaching` true)
  (`AudioComponent.Play` (`self.Audio`) 0.0)
  (set `self.overlap_count` (+ (`self.overlap_count`) 1)))

(event `self.trigger_zone.OnComponentEndOverlap`
  (params (OverlappedComponent :type "PrimitiveComponent Object Reference") (OtherActor :type "Actor Object Reference") (OtherComp :type "PrimitiveComponent Object Reference") (OtherBodyIndex :type Integer))
  ;[1 1 1] trigger_zone checks if train's Box collision component overlaps
  (cast `/Game/Blueprints/train` OtherActor)
  (bind _output_get (set `self.overlap_count` (+ (`self.overlap_count`) -1)))
  (if (== _output_get 0)
    (set `self.approaching` false)
    (`AudioComponent.Stop` (`self.Audio`))))

(event `self.ReceiveTick`
  (params (DeltaSeconds :type "Float (single-precision)"))
  (bind _returnvalue_x (`KismetMathLibrary.BreakVector` (`self.K2_GetActorLocation`)))
  (bind _returnvalue_x_2 (`KismetMathLibrary.BreakVector` (`self.K2_GetActorLocation`)))
  (bind _returnvalue_x_3 (`KismetMathLibrary.BreakVector` (`self.K2_GetActorLocation` (`GameplayStatics.GetPlayerCharacter` 0))))
  (bind _returnvalue_x_4 (`KismetMathLibrary.BreakVector` (`self.K2_GetActorLocation` (`GameplayStatics.GetPlayerCharacter` 0))))
  (`|ExecutionSequence`
    (:`then_0`
      ;[1 1 1] train warning lights-- alternate L and R emission
      (if (`self.approaching`)
        (if (not (`self.in_progress`))
          (set `self.in_progress` true)
          (bind (_direction _newtrack_0) (`Timeline|Timeline_0` :!via `PlayFromStart`)
            (:`Update`
              (if (<= _newtrack_0 0.5)
                (`MaterialInstanceDynamic.SetScalarParameterValue` (`self.emissive_mat`) "emissive_strength" (`self.lit`))
                (`MaterialInstanceDynamic.SetScalarParameterValue` (`self.emissive_mat_2`) "emissive_strength" (`self.dim`))
                (else
                  (`MaterialInstanceDynamic.SetScalarParameterValue` (`self.emissive_mat`) "emissive_strength" (`self.dim`))
                  (`MaterialInstanceDynamic.SetScalarParameterValue` (`self.emissive_mat_2`) "emissive_strength" (`self.lit`)))))
            (:`Finished`
              (set `self.in_progress` false))))
        (else
          (`MaterialInstanceDynamic.SetScalarParameterValue` (`self.emissive_mat`) "emissive_strength" (`self.dim`))
          (`MaterialInstanceDynamic.SetScalarParameterValue` (`self.emissive_mat_2`) "emissive_strength" (`self.dim`))
          (set `self.in_progress` false))))
    (:`then_1`
      (if (and (< _returnvalue_x _returnvalue_x_4) (> (- (`KismetMathLibrary.Abs` _returnvalue_x_3) (`KismetMathLibrary.Abs` _returnvalue_x_2)) 1000.0))
        (`self.K2_DestroyActor`)))))

(fn `UserConstructionScript`)