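; A truck actor that drives in a straight line and removes itself after covering a set distance.
; Each tick it moves along its negative local X axis, scaled by ForwardSpeed, Multiplier and frame time, and accumulates the distance moved.
; It destroys itself once that distance passes the limit.
; Its engine noise audio stops at BeginPlay, and the Play call is never executed.
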(event `self.ReceiveBeginPlay`
  ;[1 1 1] engine noise
  (`AudioComponent.Stop` (`self.Audio`)))

(event `self.ReceiveTick`
  (params (DeltaSeconds :type "Float (single-precision)"))
  (bind _returnvalue (* (* DeltaSeconds (`self.forwardSpeed`)) (`self.multiplier`)))
  (set `self.distance_moved` (+ (`self.distance_moved`) _returnvalue))
  (`self.K2_AddActorLocalOffset` (`KismetMathLibrary.MakeVector` (* _returnvalue -1.0)))
  (if (>= (`KismetMathLibrary.Abs` (`self.distance_moved`)) 7000.0)
    (`self.K2_DestroyActor`)))

(fn `UserConstructionScript`)