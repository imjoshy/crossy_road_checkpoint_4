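; Player pawn that moves forward, backward and sideways from axis input, without using a movement component in its graph.
; The Forward and Left/Right axes add Speed-scaled movement input along the actor's forward and right vectors.
; Tick consumes that vector, scales it by delta time and applies it as a swept offset, passing the world-space vector as a local-space delta.
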(event `self.ReceiveTick`
  (params (DeltaSeconds :type "Float (single-precision)"))
  ;[1 1 1] Frame-rate independent movement
  (bind _returnvalue (`self.ConsumeMovementInputVector`)) ; Get offset
  (`self.K2_AddActorLocalOffset` (* _returnvalue DeltaSeconds) true) ; Actually move the player
)

(event `InputAxis|Forward`
  (params (AxisValue :type "Float (single-precision)"))
  ;[1 1 1] Able to move forward and backward
  (`self.AddMovementInput` (`self.GetActorForwardVector`) (* AxisValue (`self.Speed`))))

(event `InputAxis|Left/Right`
  (params (AxisValue :type "Float (single-precision)"))
  ;[1 1 1] Able to move right and left
  (`self.AddMovementInput` (`self.GetActorRightVector`) (* AxisValue (`self.Speed`))))

(fn `UserConstructionScript`)