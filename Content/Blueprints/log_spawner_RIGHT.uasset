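; Right-side log spawner actor that keeps one Log in play at its location.
; Each Tick it checks the stored Log's LogExists flag and, when false, spawns a rotated, scaled-up replacement at an offset from itself.
; The new Log becomes the stored reference, is flagged as existing and receives a random negative Multiplier, presumably setting its speed and direction.
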(event `self.ReceiveTick`
  (params (DeltaSeconds :type "Float (single-precision)"))
  (bind (_returnvalue_x _returnvalue_y _returnvalue_z) (`KismetMathLibrary.BreakVector` (`self.K2_GetActorLocation`)))
  (if (not (`/Game/Blueprints/log.log_exists` (`self.log_ref`)))
    (bind _returnvalue (`|SpawnActorFromClass` "/Game/Blueprints/log.log_C" (`KismetMathLibrary.MakeTransform` (`KismetMathLibrary.MakeVector` (- _returnvalue_x 120.0) _returnvalue_y (- _returnvalue_z 125.0)) (struct :`Yaw` 90.0 :`Roll` 90.0) (50.0 50.0 50.0)) "Undefined" "OverrideRootScale" null null))
    (set `self.log_ref` _returnvalue)
    (set `/Game/Blueprints/log.log_exists` true _returnvalue)
    (set `/Game/Blueprints/log.multiplier` (`KismetMathLibrary.RandomFloatInRange` -1.0 -1.5) _returnvalue)))

(fn `UserConstructionScript`)