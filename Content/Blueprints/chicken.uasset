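; Player chicken character for a Crossy Road-style game, hopping through road, train and water hazards.
; Input hops use LaunchCharacter, with Timelines holding a lock against spam, turning the chicken and triggering random clucks; a counter caps backward hops.
; Vehicle and train overlaps squash or attach the chicken with particles, while Tick detects falling into water.
; All deaths reach GameOver, which detaches the camera spring arm and shows a cause-specific widget.
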(event `self.ReceiveTick`
  (params (DeltaSeconds :type "Float (single-precision)"))
  (bind (_returnvalue_x _returnvalue_y) (`KismetMathLibrary.BreakVector` (`self.K2_GetActorLocation`)))
  (bind (_returnvalue_x_2 _returnvalue_y_2 _returnvalue_z) (`KismetMathLibrary.BreakVector` (`self.K2_GetActorLocation` (`GameplayStatics.GetPlayerCharacter` 0))))
  ;[1 1 1] Record character x location and get char ref -- delete things too far back -- y for furthest left and right movement -- if taken past, stop camera and GAME OVER
  (`PlayerController.SetAudioListenerOverride` (`GameplayStatics.GetPlayerController` 0) (`self.Mesh`) (`self.K2_GetActorLocation`) (`self.K2_GetActorRotation`))
  (set `self.ch_loc_x` _returnvalue_x)
  (set `self.ch_loc_y` _returnvalue_y)
  ;[1 1 1] If character falls below water
  (if (<= _returnvalue_z 25.0)
    (`MovementComponent.SetPlaneConstraintNormal` (`self.CharacterMovement`) (0.0 0.0 1.0))
    (`self.drown`)))

(event `InputAction|Forward`
  (params (Key :type "Key Structure"))
  (bind (_returnvalue_x _returnvalue_y) (`KismetMathLibrary.BreakVector` (* (`self.GetActorForwardVector`) (`self.speed`))))
  ;[1 1 1] Character hops forward
  (:`Pressed`
    (if (not (`self.lock`))
      (`self.LaunchCharacter` (`KismetMathLibrary.MakeVector` _returnvalue_x _returnvalue_y (`self.jmp_height`)))
      (set `self.lock` true)
      (`Timeline|Timeline_3` :!via `PlayFromStart`
        (:`Finished`
          (set `self.lock` false) ; Unlock jump after action
          (`self.play_sound`)
          ;[1 1 1] character can only move 3 spaces back
          (if (not (== (`self.back_count`) 0))
            (set `self.back_count` (- (`self.back_count`) 1))))))))

(event `InputAction|Back`
  (params (Key :type "Key Structure"))
  (bind (_returnvalue_roll _returnvalue_pitch _returnvalue_yaw) (`KismetMathLibrary.BreakRotator` (`self.K2_GetActorRotation`)))
  ;[1 1 1] Do nothing if character already moved 3 spaces back
  (:`Pressed`
    (if (not (== (`self.back_count`) (`self.max_backs`)))
      (set `self.back_count` (+ (`self.back_count`) 1))
      ;[1 1 1] Rotating and hopping back
      (if (not (`self.lock`))
        (`self.LaunchCharacter` (`KismetMathLibrary.MakeVector` (* (`self.speed`) -1.0) 0.0 (`self.jmp_height`)))
        (set `self.lock` true) ; Lock jump to prevent spam
        (bind (_direction _0_1) (`Timeline|Timeline_2` :!via `PlayFromStart`)
          (:`Update`
            (`self.K2_SetActorRotation` (`KismetMathLibrary.RLerp` (`self.K2_GetActorRotation`) (`KismetMathLibrary.MakeRotator` _returnvalue_roll _returnvalue_pitch (select `int` (`KismetMathLibrary.RandomIntegerInRange` 0 1) :`0` (+ _returnvalue_yaw 180.0) :`1` (- _returnvalue_yaw 180.0))) _0_1 true)))
          (:`Finished`
            (`self.play_sound`)
            (set `self.lock` false) ; Unlock jump after action
          ))))))

(event `InputAction|Left`
  (params (Key :type "Key Structure"))
  (bind (_returnvalue_roll _returnvalue_pitch _returnvalue_yaw) (`KismetMathLibrary.BreakRotator` (`self.K2_GetActorRotation`)))
  ;[1 1 1] Rotating and hopping left
  (:`Pressed`
    (if (not (`self.lock`))
      (`self.LaunchCharacter` (`KismetMathLibrary.MakeVector` 0.0 (* (`self.speed`) -1.0) (`self.jmp_height`)))
      (set `self.lock` true) ; LOCK jump to prevent spam
      (bind (_direction _0_1) (`Timeline|Timeline_0` :!via `PlayFromStart`)
        (:`Update`
          (`self.K2_SetActorRotation` (`KismetMathLibrary.RLerp` (`self.K2_GetActorRotation`) (`KismetMathLibrary.MakeRotator` _returnvalue_roll _returnvalue_pitch (- _returnvalue_yaw 90.0)) _0_1 true)))
        (:`Finished`
          (`self.play_sound`)
          (set `self.lock` false) ; Unlock jump after action
        )))))

(event `InputAction|Right`
  (params (Key :type "Key Structure"))
  (bind (_returnvalue_roll _returnvalue_pitch _returnvalue_yaw) (`KismetMathLibrary.BreakRotator` (`self.K2_GetActorRotation`)))
  ;[1 1 1] Rotating and hopping right
  (:`Pressed`
    (if (not (`self.lock`))
      (`self.LaunchCharacter` (`KismetMathLibrary.MakeVector` 0.0 (`self.speed`) (`self.jmp_height`)))
      (set `self.lock` true) ; Lock jump to prevent spam
      (bind (_direction _0_1) (`Timeline|Timeline_1` :!via `PlayFromStart`)
        (:`Update`
          (`self.K2_SetActorRotation` (`KismetMathLibrary.RLerp` (`self.K2_GetActorRotation`) (`KismetMathLibrary.MakeRotator` _returnvalue_roll _returnvalue_pitch (+ _returnvalue_yaw 90.0)) _0_1 true)))
        (:`Finished`
          (`self.play_sound`)
          (set `self.lock` false) ; Unlock jump after action
        )))))

(event `self.car_col.OnComponentBeginOverlap`
  (params (OverlappedComponent :type "PrimitiveComponent Object Reference") (OtherActor :type "Actor Object Reference") (OtherComp :type "PrimitiveComponent Object Reference") (OtherBodyIndex :type Integer) (bFromSweep :type Boolean) (SweepResult :type "HitResult Structure (by ref)"))
  (cast `/Game/Blueprints/car` OtherActor)
  (`self.hit_vehicle` :!label _label))

(event `self.police_car_col.OnComponentBeginOverlap`
  (params (OverlappedComponent :type "PrimitiveComponent Object Reference") (OtherActor :type "Actor Object Reference") (OtherComp :type "PrimitiveComponent Object Reference") (OtherBodyIndex :type Integer) (bFromSweep :type Boolean) (SweepResult :type "HitResult Structure (by ref)"))
  (cast `/Game/Blueprints/police_car` OtherActor)
  (goto _label))

(event `self.truck1_col.OnComponentBeginOverlap`
  (params (OverlappedComponent :type "PrimitiveComponent Object Reference") (OtherActor :type "Actor Object Reference") (OtherComp :type "PrimitiveComponent Object Reference") (OtherBodyIndex :type Integer) (bFromSweep :type Boolean) (SweepResult :type "HitResult Structure (by ref)"))
  (cast `/Game/Blueprints/truck_1` OtherActor)
  (goto _label))

(event `self.truck2_col.OnComponentBeginOverlap`
  (params (OverlappedComponent :type "PrimitiveComponent Object Reference") (OtherActor :type "Actor Object Reference") (OtherComp :type "PrimitiveComponent Object Reference") (OtherBodyIndex :type Integer) (bFromSweep :type Boolean) (SweepResult :type "HitResult Structure (by ref)"))
  (cast `/Game/Blueprints/truck_2` OtherActor)
  (goto _label))

(event `self.train_col.OnComponentBeginOverlap`
  (params (OverlappedComponent :type "PrimitiveComponent Object Reference") (OtherActor :type "Actor Object Reference") (OtherComp :type "PrimitiveComponent Object Reference") (OtherBodyIndex :type Integer) (bFromSweep :type Boolean) (SweepResult :type "HitResult Structure (by ref)"))
  (bind _astrain (cast `/Game/Blueprints/train` OtherActor))
  (set `self.train_hit_ref` _astrain)
  (if (not (`self.hit`))
    (set `self.hit` true)
    (`self.hit_train`)))

(fn `drown`
  (bind (_returnvalue_x _returnvalue_y _returnvalue_z) (`KismetMathLibrary.BreakVector` (`self.K2_GetActorLocation` (`GameplayStatics.GetPlayerCharacter` 0))))
  (if (not (`self.is_dead`))
    (`GameplayStatics.SpawnEmitterAtLocation` "/Game/migrated/ParticleSystems/PS_splash.PS_splash" (`KismetMathLibrary.MakeVector` _returnvalue_x _returnvalue_y (+ _returnvalue_z 10.0)))
    (set `self.drowned` true)
    (`self.game_over`)))

(fn `game_over`
  (bind _returnvalue (`GameplayStatics.GetPlayerController` 0))
  (bind _returnvalue_2 (`GameplayStatics.GetPlayerController` 0))
  (if (not (`self.is_dead`))
    (set `self.is_dead` true)
    (`GameplayStatics.SpawnSoundAttached` "/Game/Assets/sounds/chicken/chicken_3.chicken_3" (`self.MediaSound`) "None" (0.0 0.0 0.0) (struct) "KeepRelativeOffset" false 5.0 1.0 0.0 null "/Game/Assets/sounds/SoundConcurrency.SoundConcurrency")
    (`SceneComponent.K2_DetachFromComponent` (`self.SpringArm`) "KeepWorld" "KeepRelative" "KeepWorld" false)
    (if (`self.drowned`)
      (bind _returnvalue_3 (`|CreateWidget` "/Game/Blueprints/BP_game_over_drown.BP_game_over_drown_C"))
      (`UserWidget.AddToViewport` _returnvalue_3 0)
      (`WidgetBlueprintLibrary.SetInputMode_UIOnlyEx` _returnvalue_2 _returnvalue_3 "LockOnCapture")
      (set `PlayerController.bShowMouseCursor` true _returnvalue_2)
      (else
        (bind _returnvalue_4 (`|CreateWidget` "/Game/Blueprints/BP_game_over_vehicle_train.BP_game_over_vehicle_train_C"))
        (`UserWidget.AddToViewport` _returnvalue_4 0)
        (`WidgetBlueprintLibrary.SetInputMode_UIOnlyEx` _returnvalue _returnvalue_4 "LockOnCapture")
        (set `PlayerController.bShowMouseCursor` true _returnvalue)))))

(fn `hit_train`
  (bind (_returnvalue_x _returnvalue_y _returnvalue_z) (`KismetMathLibrary.BreakVector` (`SceneComponent.K2_GetComponentScale` (`self.StaticMesh`))))
  (bind (_returnvalue_x_2 _returnvalue_y_2 _returnvalue_z_2) (`KismetMathLibrary.BreakVector` (`self.K2_GetActorLocation` (`GameplayStatics.GetPlayerCharacter` 0))))
  (`|ExecutionSequence`
    (:`then_0`
      (`self.game_over`))
    (:`then_1`
      (`self.K2_AttachToActor` (`self.train_hit_ref`) "None" "KeepWorld" "KeepWorld" "KeepWorld"))
    (:`then_2`
      (`SceneComponent.SetWorldScale3D` (`self.StaticMesh`) (`KismetMathLibrary.MakeVector` _returnvalue_x (* _returnvalue_y 1.5) (* _returnvalue_z 1.5)))
      (`GameplayStatics.SpawnEmitterAtLocation` "/Game/migrated/ParticleSystems/PS_train.PS_train" (`KismetMathLibrary.MakeVector` _returnvalue_x_2 _returnvalue_y_2 _returnvalue_z_2)))))

(fn `hit_vehicle`
  (bind (_returnvalue_x _returnvalue_y _returnvalue_z) (`KismetMathLibrary.BreakVector` (`SceneComponent.K2_GetComponentScale` (`self.StaticMesh`))))
  (bind (_returnvalue_x_2 _returnvalue_y_2 _returnvalue_z_2) (`KismetMathLibrary.BreakVector` (`self.K2_GetActorLocation` (`GameplayStatics.GetPlayerCharacter` 0))))
  (bind (_returnvalue_x_3 _returnvalue_y_3 _returnvalue_z_3) (`KismetMathLibrary.BreakVector` (`self.K2_GetActorLocation` (`GameplayStatics.GetPlayerCharacter` 0))))
  (if (not (`self.hit`))
    (set `self.hit` true)
    (`GameplayStatics.SpawnEmitterAtLocation` "/Game/migrated/ParticleSystems/PS_vehicle.PS_vehicle" (`KismetMathLibrary.MakeVector` (- _returnvalue_x_2 5.0) (- _returnvalue_y_2 5.0) (- _returnvalue_z_2 5.0)))
    (`|ExecutionSequence`
      (:`then_0`
        (`SceneComponent.SetWorldScale3D` (`self.StaticMesh`) (`KismetMathLibrary.MakeVector` (* _returnvalue_x 3.0) (* _returnvalue_y 0.25) _returnvalue_z))
        (`self.game_over`))
      (:`then_1`
        (`self.K2_AddActorLocalOffset` (`KismetMathLibrary.MakeVector` 0.0 0.0 (+ _returnvalue_z_3 -60.0)))
        (`MovementComponent.SetPlaneConstraintNormal` (`self.CharacterMovement`) (0.0 0.0 1.0))))))

(fn `play_sound`
  ;[1 1 1] cluck cluck -- 2/5 chance of no sound
  (`GameplayStatics.SpawnSoundAttached` (select `int` (`KismetMathLibrary.RandomIntegerInRange` 0 4) :`0` "/Game/Assets/sounds/chicken/chicken_1.chicken_1" :`1` "/Game/Assets/sounds/chicken/chicken_1.chicken_1" :`2` "/Game/Assets/sounds/chicken/chicken_2.chicken_2" :`3` null :`4` null :!type "SoundBase Object Reference") (`self.MediaSound`) "None" (0.0 0.0 0.0) (struct) "KeepRelativeOffset" false 5.0 1.0 0.0 null "/Game/Assets/sounds/SoundConcurrency.SoundConcurrency"))

(fn `UserConstructionScript`)